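; BP_DialogueSpawner is a trigger actor that shows timed dialogue and runs a damage countdown while its sphere is overlapped.
; It creates a W_Dialogue widget at BeginPlay, adds it on overlap, and removes it and resets the index on exit.
; A Delay loop advances DialogueLines every second without an exit check.
; A flag-gated loop repeatedly lowers the actor's own Health variable, printing it as the player's.
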(event OnComponentBeginOverlap(Sphere)
  (params (OverlappedComponent :type Primitive%20Component%20Object%20Reference) (OtherActor :type Actor%20Object%20Reference) (OtherComp :type Primitive%20Component%20Object%20Reference) (OtherBodyIndex :type Integer) (bFromSweep :type Boolean) (SweepResult :type Hit%20Result%20Structure%20%28by%20ref%29))
  (bind _dialoguewidget (Variables|Default|GetDialogueWidget))
  (bind _index (Variables|Default|Getindex))
  (Variables|Default|SetPlayerIsInTrigger true)
  (CallFunction|DamagePlayer)
  (UserInterface|Viewport|AddtoViewport _dialoguewidget 0)
  (Utilities|FlowControl|Delay 1.0 :!label _label)
  (Math|Integer|IncrementInt _index
    (:%20%20
      (Rendering|Components|TextRender|SetText (Variables|/Game/W_Dialogue.W_Dialogue_C|GetTextBlock_3 _dialoguewidget) (Utilities|Array|Get(acopy) (Variables|Default|GetDialogueLines) _index))
      (goto _label))))

(event OnComponentEndOverlap(Sphere)
  (params (OverlappedComponent :type Primitive%20Component%20Object%20Reference) (OtherActor :type Actor%20Object%20Reference) (OtherComp :type Primitive%20Component%20Object%20Reference) (OtherBodyIndex :type Integer))
  (bind _dialoguewidget (Variables|Default|GetDialogueWidget))
  (Variables|Default|SetPlayerIsInTrigger false)
  (Widget|RemovefromParent _dialoguewidget)
  (Rendering|Components|TextRender|SetText (Variables|/Game/W_Dialogue.W_Dialogue_C|GetTextBlock_3 _dialoguewidget) "")
  (Variables|Default|Setindex 0))

(event Custom|Damage%20player
  (if (Variables|Default|GetPlayerIsInTrigger) :!label _label
    (bind _output_get (Variables|Default|Sethealth (- (Variables|Default|Gethealth) 5)))
    (Development|PrintText (Utilities|Text|FormatText "{playerName} now has {health} health." _output_get (Utilities|GetDisplayName (Game|GetPlayerCharacter 0))))
    (Utilities|FlowControl|Delay 0.2)
    (goto _label)))

(event EventBeginPlay
  (bind _returnvalue (UserInterface|CreateWidget "/Game/W_Dialogue.W_Dialogue_C"))
  (Variables|Default|SetDialogueWidget _returnvalue)
  (Input|EnableInput (Game|GetPlayerController 0)))

(event Collision|EventActorBeginOverlap
  (params (OtherActor :type Actor%20Object%20Reference)))

(event EventTick
  (params (DeltaSeconds :type Float%20%28single-precision%29)))

(fn ConstructionScript)