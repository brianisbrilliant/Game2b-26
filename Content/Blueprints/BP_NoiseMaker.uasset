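; BP_NoiseMaker is an actor that emits a repeating multi-sensory pulse at its location, starting on BeginPlay.
; Each pulse fires attenuated force feedback, a legacy camera shake from its CameraShakeSource on player 0's camera manager, a sine ping sound and a directional burst effect above the actor.
; A two-second Delay follows, then it prints "Boom" and loops back indefinitely.
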(event EventBeginPlay
  (ForceFeedback|SpawnForceFeedbackatLocation "/Game/ForceFeedback/FFE_Interact.FFE_Interact" (Transformation|GetActorLocation) "0, 0, 0" false 1.0 0.0 "/Game/ForceFeedback/FFA_Default.FFA_Default" :!label _label)
  (Class|LegacyCameraShake|StartLegacyCameraShakefromSource (Game|GetPlayerCameraManager 0) 0 (Variables|Default|GetCameraShakeSource) 1.0 "CameraLocal" "0, 0, 0")
  (Audio|PlaySoundatLocation "/Engine/EngineSounds/1kSineTonePing.1kSineTonePing" (Transformation|GetActorLocation) "0, 0, 0" 1.0 1.0 0.0 "/Game/Audio/ATT_Default.ATT_Default" 0 0 0)
  (Niagara|SpawnSystematLocation "/Niagara/DefaultAssets/Templates/Systems/DirectionalBurst.DirectionalBurst" (+ (Transformation|GetActorLocation) "0.000000,0.000000,100.000000") "90.000000,0.000000,0.000000")
  (Utilities|FlowControl|Delay 2.0)
  (Development|PrintText "Boom")
  (goto _label))

(fn ConstructionScript)